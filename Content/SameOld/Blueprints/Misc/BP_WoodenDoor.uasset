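; BP_WoodenDoor is a level exit door that rises or lowers to let the player reach the next level.
; When its C++ OpenDoor component broadcasts OnOpenRequest, a timeline drives the actor's Z position while a sound and a level sequence play, with input and HUD disabled.
; BP_Alex is made invulnerable and the gamemode's DoorIsOpening flag is set during the opening, both reverting one second after it finishes.
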(event OnOpenRequest(OpenDoor)
  (bind _returnvalue (Game|GetGameMode))
  (bind _returnvalue_2 (Transformation|GetActorLocation))
  (bind _returnvalue_3 (Game|GetPlayerController 0))
  (bind _returnvalue_4 (Pawn|GetControlledPawn _returnvalue_3))
  (bind _asbp_main_gamemode (Utilities|Casting|CastToBP_MainGamemode _returnvalue))
  (bind _asbp_alex (Utilities|Casting|CastToBP_Alex _returnvalue_4))
  ;[1 1 1] Runs when OnOpenRequest from the c++ component OpenDoor is broadcasted. Moves the door so the player can get to the next level
  (bind _outactor (Sequencer|Player|CreateLevelSequencePlayer "/Game/SameOld/UI/LevelSequence_DoorOpens.LevelSequence_DoorOpens" (Utilities|Struct|MakeMovieSceneSequencePlaybackSettings 0 1.0 false 0.0 false true true false true false false 0)))
  (Sequencer|Player|Play (Variables|/Script/LevelSequence.LevelSequenceActor|GetSequencePlayer _outactor) :!class /Script/MovieScene.MovieSceneSequencePlayer)
  (Class|MyCharacter|SetCanGetHurt _asbp_alex false)
  (Audio|PlaySoundatLocation "/Game/Audio/Misc/S_WoodenDoor.S_WoodenDoor" (Transformation|GetActorLocation) "0, 0, 0" 1.0 1.0 0.0 0 0 0)
  (Variables|/Game/SameOld/Blueprints/Gamemodes/BP_MainGamemode.BP_MainGamemode_C|SetdoorIsOpening _asbp_main_gamemode true)
  (bind _opendoor (Timeline|Timeline_0 Play)
    (:Update
      (Transformation|SetActorLocation (Math|Vector|MakeVector (.x _returnvalue_2) (.y _returnvalue_2) _opendoor) false false))
    (:Finished
      (Sequencer|Player|Stop (Variables|/Script/LevelSequence.LevelSequenceActor|GetSequencePlayer _outactor) :!class /Script/MovieScene.MovieSceneSequencePlayer)
      (Utilities|FlowControl|Delay 1.0)
      (Class|MyCharacter|SetCanGetHurt _asbp_alex true)
      (Variables|/Game/SameOld/Blueprints/Gamemodes/BP_MainGamemode.BP_MainGamemode_C|SetdoorIsOpening _asbp_main_gamemode false))))

(fn ConstructionScript
  (|CallParentFunction))