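; BP_MainGamemode is the gamemode that sets up a level and watches for its win condition.
; On BeginPlay it creates the WBP_HUD widget, adds it to the viewport and plays the level sound.
; Every Tick, if CheckIfNextLevel passes and no enemies remain, it compares the current level name to Level2Name and opens CutScene2 on a match.
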(event EventBeginPlay
  ;[1 1 1] Creates HUD and shows it on the screen
  (bind _returnvalue (UserInterface|CreateWidget "/Game/SameOld/UI/WBP_HUD.WBP_HUD_C" (Game|GetPlayerController 0)))
  (UserInterface|Viewport|AddtoViewport _returnvalue 0)
  (Audio|PlaySound2D "/Game/Audio/Music/S_Level.S_Level" 1.0 1.0 0.0 0 0))

(event EventTick
  (params (DeltaSeconds :type Float%20%28single-precision%29))
  ;[1 1 1] Checks if you win the game
  (if (Class|Gruppe21GameModeBase|CheckifNextLevel)
    (if (== (Class|Gruppe21GameModeBase|GetNumberOfEnemies) 0)
      (bind _returnvalue (Game|GetCurrentLevelName true))
      (if (Utilities|Name|Equal(Name) (Utilities|String|StringToName _returnvalue) (Variables|Game|GetLevel2Name))
        (Game|OpenLevel(byName) "CutScene2")))))

(fn ConstructionScript)