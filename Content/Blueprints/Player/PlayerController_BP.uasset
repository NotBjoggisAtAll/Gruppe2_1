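; Player controller that turns the controlled pawn to face the mouse cursor, as in a top-down aiming setup.
; Every tick it traces under the cursor against a single object type with complex collision.
; On a hit, it computes a look-at rotation from the pawn to the hit point and applies only the yaw, keeping the pawn level.
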(event EventTick
  (params (DeltaSeconds :type Float%20%28single-precision%29))
  (bind _array (Utilities|Array|MakeArray "ObjectTypeQuery7"))
  (bind _hitresult (Class|PlayerController|GetHitResultUnderCursorforObjects _array true))
  (bind (_bblockinghit _binitialoverlap _time _distance _location) (Collision|BreakHitResult _hitresult))
  (Utilities|FlowControl|Sequence
    (:then_0
      (if _bblockinghit
        (Transformation|SetActorRotation (Pawn|GetControlledPawn) (Math|Rotator|MakeRotator 0.0 0.0 (.Yaw (Math|Rotator|BreakRotator (Math|Rotator|FindLookatRotation (Transformation|GetActorLocation (Pawn|GetControlledPawn)) _location)))))))))

(fn ConstructionScript)