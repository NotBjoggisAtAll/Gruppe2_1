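; Player Blueprint that handles damage, pickups and tracking of objects between the camera and the player.
; Overlaps with enemies or Enemy3 projectiles cost health with a brief invulnerability window, destroying the player at zero.
; Pickups restore capped health or temporarily change fire rate.
; A looping timer multi-line traces from camera to player, refreshing the IsSeen flag on SuperDuperMaterialClass hits, likely for see-through walls.
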(event Collision|EventActorBeginOverlap
  (params (OtherActor :type Actor%20Object%20Reference))
  (bind _asenemy_3projectile_bp (Utilities|Casting|CastToEnemy3Projectile_BP OtherActor)
    (:then
      (Actor|DestroyActor _asenemy_3projectile_bp)
      (if (Variables|Default|GetCanPlayerGetDamaged) :!label _label
        (bind _output_get (Variables|Default|SetHealth (- (Variables|Default|GetHealth) 100)))
        (Variables|Default|SetCanPlayerGetDamaged false)
        (if (== _output_get 0)
          (Actor|DestroyActor)
          (else
            (Utilities|FlowControl|Delay 2.0)
            (Variables|Default|SetCanPlayerGetDamaged true)
            (Development|PrintString "damage")))))
    (:CastFailed
      (Utilities|Casting|CastToMyEnemy OtherActor
        (:then
          (goto _label))
        (:CastFailed
          (bind _asmy_fire_rate_up_bp (Utilities|Casting|CastToMyFireRateUp_BP OtherActor)
            (:then
              (Actor|DestroyActor _asmy_fire_rate_up_bp)
              (Variables|Default|SetFireRate 0.1)
              (Utilities|FlowControl|Delay 5.0)
              (Variables|Default|SetFireRate 1.0))
            (:CastFailed
              (bind _asmy_health_bp (Utilities|Casting|CastToMyHealth_BP OtherActor))
              (Actor|DestroyActor _asmy_health_bp)
              (if (< (+ (Variables|Default|GetHealth) 200) 500)
                (Variables|Default|SetHealth (+ (Variables|Default|GetHealth) 200))
                (else
                  (Variables|Default|SetHealth 500))))))))))

(event EventBeginPlay
  (Utilities|Time|SetTimerbyFunctionName 0 "UpdateWalls" 0.1 true))

(fn ConstructionScript)

(fn UpdateWalls
  (bind _objectsseen (Variables|Default|GetObjectsSeen))
  (for _array_element _objectsseen
    (Variables|/Game/Blueprints/FadedMaterials/SuperDuperMaterialClass.SuperDuperMaterialClass_C|SetIsSeen _array_element false))
  (Utilities|Array|Clear _objectsseen)
  (bind (_outhits _returnvalue) (Collision|MultiLineTraceByChannel (Transformation|GetWorldLocation (Variables|Default|GetCameraComponent)) (Transformation|GetActorLocation) "TraceTypeQuery1" false 0 "None"))
  (if _returnvalue
    (for _array_element_2 _outhits
      (if (.bSuccess (Utilities|Casting|CastToSuperDuperMaterialClass (.hitactor _array_element_2)))
        (Utilities|Array|AddUnique (Variables|Default|GetObjectsSeen) (.AsSuper%20Duper%20Material%20Class (Utilities|Casting|CastToSuperDuperMaterialClass (.hitactor _array_element_2))))
        (Variables|/Game/Blueprints/FadedMaterials/SuperDuperMaterialClass.SuperDuperMaterialClass_C|SetIsSeen (.AsSuper%20Duper%20Material%20Class (Utilities|Casting|CastToSuperDuperMaterialClass (.hitactor _array_element_2))) true)))))