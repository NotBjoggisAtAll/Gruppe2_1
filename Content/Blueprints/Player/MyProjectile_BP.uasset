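; MyProjectile_BP is a player projectile Blueprint containing pickup-drop logic for enemy hits, which is currently disconnected and never runs.
; The Destroyed event and construction script are empty.
; The orphaned nodes check EnemyHit, roll a roughly one-in-five drop chance, then spawn a half-scale fire-rate or health pickup at EnemyDeath, favoring health two to one.
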(event EventDestroyed)

(fn ConstructionScript)