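; Player character Blueprint for Alex, handling wall see-through, damage feedback, enemy crowding and the pause and game-over menus.
; A looping timer line-traces from camera to player, setting IsSeen on intervening BP_FadedMaterialsClass actors.
; An overlap component tracks nearby enemies, and Tick switches two capsule collision channels to Overlap when crowded, preventing the player getting stuck.
; Enemy or moth-projectile damage plays a timeline-driven post-process flash when the player can be hurt.
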(event Game|Damage|EventAnyDamage
  (params (Damage :type Float%20%28single-precision%29) (DamageType :type Damage%20Type%20Object%20Reference) (InstigatedBy :type Controller%20Object%20Reference) (DamageCauser :type Actor%20Object%20Reference))
  ;[1 1 1] Makes the screen red to indicate that you took damage
  (if (and (or (.bSuccess (Utilities|Casting|CastToMyEnemy DamageCauser)) (.bSuccess (Utilities|Casting|CastToBP_MothProjectile DamageCauser))) (Class|MyCharacter|GetCanGetHurt))
    (bind _blendweight (Timeline|Timeline_0 PlayFromStart)
      (:Update
        (Variables|/Script/Engine.PostProcessComponent|SetBlendWeight (Variables|Default|GetPostProcess) _blendweight)))))

(event EventBeginPlay
  ;[1 1 1] Enables the UpdateWalls function so walls between you and the camera is transparent
  (Utilities|Time|SetTimerbyFunctionName 0 "UpdateWalls" 0.1 true))

(event Input|ActionEvents|InputActionPauseGame
  (params (Key :type Key%20Structure))
  ;[1 1 1] Pause Game Function
  (:Pressed
    (CallFunction|PauseGame)))

(event OnComponentBeginOverlap(EnemyDetecter)
  (params (OverlappedComponent :type Primitive%20Component%20Object%20Reference) (OtherActor :type Actor%20Object%20Reference) (OtherComp :type Primitive%20Component%20Object%20Reference) (OtherBodyIndex :type Integer) (bFromSweep :type Boolean) (SweepResult :type Hit%20Result%20Structure%20%28by%20ref%29))
  (bind (_asmy_enemy _bsuccess) (Utilities|Casting|CastToMyEnemy OtherActor))
  ;[1 1 1] Detects when enemies gets to close to the player and adds them to an array
  (if _bsuccess
    (Utilities|Array|Add (Variables|Default|GetEnemiesNear) _asmy_enemy)))

(event OnComponentEndOverlap(EnemyDetecter)
  (params (OverlappedComponent :type Primitive%20Component%20Object%20Reference) (OtherActor :type Actor%20Object%20Reference) (OtherComp :type Primitive%20Component%20Object%20Reference) (OtherBodyIndex :type Integer))
  (bind (_asmy_enemy _bsuccess) (Utilities|Casting|CastToMyEnemy OtherActor))
  ;[1 1 1] Detects when enemies die or move away from the player and removes them from the array
  (if _bsuccess
    (Utilities|Array|RemoveItem (Variables|Default|GetEnemiesNear) _asmy_enemy)))

(event EventTick
  (params (DeltaSeconds :type Float%20%28single-precision%29))
  (bind _capsulecomponent (Variables|Default|GetCapsuleComponent))
  ;[1 1 1] Checks how many enemies that are in the array, if too many it changes the player collision to prevent the player from getting stuck
  (if (>= (Utilities|Array|Length (Variables|Default|GetEnemiesNear)) 6)
    (Collision|SetCollisionResponsetoChannel _capsulecomponent "ECC_GameTraceChannel7" "ECR_Overlap")
    (Collision|SetCollisionResponsetoChannel _capsulecomponent "ECC_GameTraceChannel5" "ECR_Overlap")
    (else
      (Utilities|FlowControl|Delay 0.5)
      (Collision|SetCollisionResponsetoChannel _capsulecomponent "ECC_GameTraceChannel7" "ECR_Block")
      (Collision|SetCollisionResponsetoChannel _capsulecomponent "ECC_GameTraceChannel5" "ECR_Block"))))

(fn ConstructionScript)

(fn UpdateWalls
  (bind _objectsseen (Variables|Default|GetObjectsSeen))
  (for _array_element _objectsseen
    (Variables|/Game/Blueprints/Misc/BP_FadedMaterialsClass.BP_FadedMaterialsClass_C|SetIsSeen _array_element false))
  (Utilities|Array|Clear _objectsseen)
  (bind (_outhits _returnvalue) (Collision|MultiLineTraceByChannel (Transformation|GetWorldLocation (Variables|Default|GetCameraComponent)) (Transformation|GetActorLocation) "TraceTypeQuery1" false 0 "None"))
  (if _returnvalue
    (for _array_element_2 _outhits
      (if (.bSuccess (Utilities|Casting|CastToBP_FadedMaterialsClass (.hitactor _array_element_2)))
        (Utilities|Array|AddUnique (Variables|Default|GetObjectsSeen) (.AsBP%20Faded%20Materials%20Class (Utilities|Casting|CastToBP_FadedMaterialsClass (.hitactor _array_element_2))))
        (Variables|/Game/Blueprints/Misc/BP_FadedMaterialsClass.BP_FadedMaterialsClass_C|SetIsSeen (.AsBP%20Faded%20Materials%20Class (Utilities|Casting|CastToBP_FadedMaterialsClass (.hitactor _array_element_2))) true)))))

(fn PauseGame
  ;[1 1 1] This pauses and unpauses the game respectively.
  (if (Variables|Default|GetIsPaused)
    (Game|SetGamePaused false)
    (Variables|Default|SetIsPaused false)
    (Widget|RemovefromParent (stale _output_get))
    (else
      (Game|SetGamePaused true)
      (bind _returnvalue (UserInterface|CreateWidget "/Game/UI/WBP_PauseMenu.WBP_PauseMenu_C"))
      (bind _output_get (Variables|Default|SetPauseScreen _returnvalue))
      (UserInterface|Viewport|AddtoViewport _output_get 0)
      (Variables|Default|SetIsPaused true))))

(fn GameOverScreen
  (Game|SetGamePaused true)
  (bind _returnvalue (UserInterface|CreateWidget "/Game/UI/WBP_GameOverMenu.WBP_GameOverMenu_C"))
  (UserInterface|Viewport|AddtoViewport _returnvalue 0))