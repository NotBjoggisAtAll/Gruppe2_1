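; Moth enemy Blueprint that periodically fires projectiles at the player.
; Tick runs into a five-second Delay, which throttles FireShot to a repeating timed shot.
; FireShot checks that the player character is valid, then spawns a half-scale Enemy3Projectile_BP facing the player, ignoring collisions.
; The muzzle offset is rotated by the player's world position vector, not by the direction from moth to player.
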(event EventTick
  (params (DeltaSeconds :type Float%20%28single-precision%29))
  (Utilities|FlowControl|Delay 5.0)
  (CallFunction|FireShot))

(fn ConstructionScript)

(fn FireShot
  (bind _returnvalue (Transformation|GetActorLocation))
  (bind _returnvalue_2 (Game|GetPlayerCharacter 0))
  (bind _returnvalue_3 (Transformation|GetActorLocation _returnvalue_2))
  ;[1 1 1] Spawn Projectile at location
  (Utilities|IsValid _returnvalue_2
    (:Is%20Valid
      (bind _returnvalue_4 (Game|SpawnActorfromClass "/Game/Blueprints/Enemies/Enemy3Projectile_BP.Enemy3Projectile_BP_C" (Math|Transform|MakeTransform (* (+ _returnvalue (Math|Vector|RotateVector (Variables|Default|GetGunOffset) (Math|Conversions|RotationFromXVector _returnvalue_3))) "1.000000,1.000000,1.000000") (Math|Rotator|FindLookatRotation _returnvalue _returnvalue_3) "0.500000,0.500000,0.500000") "AlwaysSpawn" 0 0))
      (return _returnvalue_4))))