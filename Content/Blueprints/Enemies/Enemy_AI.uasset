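; Enemy AI controller that moves an enemy toward the player or, on the level named by Level2Name, toward a defendable object.
; A looping timer started on BeginPlay calls Track Player to reissue the move order at a set interval.
; Track Player checks the current level name, then moves to the location of the first MyDefendableObject_BP found or follows the player character.
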(event EventBeginPlay
  (Utilities|Time|SetTimerbyFunctionName 0 "Track Player" (Variables|Default|GetTime%20before%20moving%20to%20Player) true))

(fn ConstructionScript)

(fn TrackPlayer
  (bind _acceptance_radius (Variables|Default|GetAcceptance%20Radius))
  (bind _returnvalue (Game|GetCurrentLevelName true))
  (if (Utilities|Name|Equal(Name) (Utilities|String|StringToName _returnvalue) (Variables|Default|GetLevel%202%20Name))
    (bind _outactors (Actor|GetAllActorsOfClass "/Game/Blueprints/MyDefendableObject_BP.MyDefendableObject_BP_C"))
    (AI|Navigation|MovetoLocation (Transformation|GetActorLocation (Utilities|Array|Get(acopy) _outactors)) _acceptance_radius true true false)
    (else
      (AI|Navigation|MovetoActor (Game|GetPlayerCharacter 0) _acceptance_radius false true))))