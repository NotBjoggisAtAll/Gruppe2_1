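; Game mode that creates the player HUD on begin play and keeps enemies spawning during the game.
; Every tick it counts MyEnemy_BP actors and, while below the maximum and off cooldown, tells a random MySpawnpoint_BP to spawn one.
; A boolean flag reset by a timer after SpawnRate seconds spaces out the spawns.
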(event EventBeginPlay
  ;[1 1 1] Creates HUD and shows it on the screen
  (bind _returnvalue (UserInterface|CreateWidget "/Game/Blueprints/HUD.HUD_C" (Game|GetPlayerController 0)))
  (UserInterface|Viewport|AddtoViewport _returnvalue 0))

(event EventTick
  (params (DeltaSeconds :type Float%20%28single-precision%29))
  (Utilities|FlowControl|Sequence
    (:then_0
      ;[1 1 1] Counts number of enemies
      (bind _outactors (Actor|GetAllActorsOfClass "/Game/Blueprints/Enemies/MyEnemy_BP.MyEnemy_BP_C"))
      (Variables|Enemies|SetNumber%20of%20Enemies (Utilities|Array|Length _outactors)))
    (:then_1
      ;[1 1 1 1 28] Selects a random spawnpoint and spawns one enemy
      (bind _outactors_2 (Actor|GetAllActorsOfClass "/Game/Blueprints/Enemies/MySpawnpoint_BP.MySpawnpoint_BP_C"))
      (if (< (Variables|Enemies|GetNumber%20of%20Enemies) (Variables|Enemies|GetMax%20Number%20Of%20Enemies))
        (if (Variables|Enemies|GetCanSpawnEnemy)
          (Class|MySpawnpoint|SpawnEnemy (Utilities|Array|Get(acopy) _outactors_2 (Math|Random|RandomIntegerinRange 0 (- (Utilities|Array|Length _outactors_2) 1))))
          (Variables|Enemies|SetCanSpawnEnemy false)
          (Utilities|Time|SetTimerbyFunctionName 0 "ResetCanSpawnEnemy" (Variables|Enemies|GetSpawn%20Rate)))))))

(fn ConstructionScript)

(fn ResetCanSpawnEnemy
  (Variables|Enemies|SetCanSpawnEnemy true))