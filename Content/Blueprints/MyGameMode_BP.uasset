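; MyGameMode_BP is a game mode Blueprint that shows the HUD and handles the win condition on the second level.
; BeginPlay creates the HUD widget for the first player and adds it to the viewport.
; Tick polls GetNextLevel, and when it is true on the level matching Level2Name, it shows a YouWin widget and pauses the game.
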(event EventBeginPlay
  ;[1 1 1] Creates HUD and shows it on the screen
  (bind _returnvalue (UserInterface|CreateWidget "/Game/UI/HUD.HUD_C" (Game|GetPlayerController 0)))
  (UserInterface|Viewport|AddtoViewport _returnvalue 0))

(event EventTick
  (params (DeltaSeconds :type Float%20%28single-precision%29))
  (if (Class|Gruppe21GameModeBase|GetNextLevel)
    (bind _returnvalue (Game|GetCurrentLevelName true))
    (if (Utilities|Name|Equal(Name) (Utilities|String|StringToName _returnvalue) (Variables|Default|GetLevel2Name))
      (bind _returnvalue_2 (UserInterface|CreateWidget "/Game/UI/YouWin.YouWin_C"))
      (UserInterface|Viewport|AddtoViewport _returnvalue_2 0)
      (Game|SetGamePaused true))))

(fn ConstructionScript)