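; BP_WoodenWall is a wall actor that fades its material when it is between the player and the camera.
; BeginPlay creates a dynamic material instance of M_Wall1 on the static mesh.
; Each Tick plays or reverses a timeline based on IsSeen, which this graph only reads, feeding the MyVisibility scalar parameter.
; Older material-swapping nodes remain in the graph but are disconnected.
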(event EventBeginPlay
  (bind _returnvalue (Rendering|Material|CreateDynamicMaterialInstance (Variables|Default|GetStaticMesh) 0 "/Game/Materials/Map/M_Wall1.M_Wall1" "None" :!class /Script/Engine.PrimitiveComponent)))

(event EventTick
  (params (DeltaSeconds :type Float%20%28single-precision%29))
  (if (Variables|Default|GetIsSeen)
    (bind _newtrack_0 (Timeline|Timeline_0 Play)
      (:Update
        _)
      (:Finished
        _))
    (Rendering|Material|SetScalarParameterValue (stale EventBeginPlay _returnvalue) "MyVisibility" _newtrack_0 :!class /Script/Engine.MaterialInstanceDynamic)
    (else
      (Timeline|Timeline_0 Reverse))))

(fn ConstructionScript)